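; BP_Pokemon is a generic, data-driven Pokémon whose skeletal mesh and animation Blueprint come from its PokemonData.
; BeginPlay applies the visuals from the current data.
; The SetPokemonData event stores new data and calls SetBPPokemonData, which reapplies mesh and animation class, with both printing the Pokémon name in Spanish debug messages.
; GetPokemonData returns the stored data.
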(event `self.ReceiveBeginPlay`
  (bind (_pokemonname _currenthealth _maxhealth _speed _moves _pokemonmesh _animationblueprint) (break `/Game/test001/PKMN_Data/Structures/S_combatPKMN` (`self.PokemonData`)))
  (`SkeletalMeshComponent.SetSkeletalMeshAsset` (`self.Mesh`) _pokemonmesh)
  (`SkeletalMeshComponent.SetAnimInstanceClass` (`self.Mesh`) _animationblueprint))

(event `/Game/test001/Blueprints/Interfaces/BPI_PokemonData.SetPokemonData`
  (params (NewPokemonData :type "/Game/test001/PKMN_Data/Structures/S_combatPKMN Structure"))
  (bind _output_get (set `self.PokemonData` NewPokemonData))
  (`self.SetBP_PokemonData` _output_get)
  (`KismetSystemLibrary.PrintString` (`KismetStringLibrary.Concat_StrStr` "Datos del Pokémon asignados en BP_Pokemon: " (`.PokemonName_2_D07B2A324EF6628628040A863E139A85` (break `/Game/test001/PKMN_Data/Structures/S_combatPKMN` _output_get)))))

(fn `GetPokemonData`
  (returns (ReturnValue :type "/Game/test001/PKMN_Data/Structures/S_combatPKMN Structure"))
  (return (`self.PokemonData`)))

(fn `SetBP_PokemonData`
  (params (NewBP_PokemonData :type "/Game/test001/PKMN_Data/Structures/S_combatPKMN Structure"))
  (bind _output_get (set `self.PokemonData` NewBP_PokemonData))
  (bind (_pokemonname _currenthealth _maxhealth _speed _moves _pokemonmesh _animationblueprint) (break `/Game/test001/PKMN_Data/Structures/S_combatPKMN` _output_get))
  (`KismetSystemLibrary.PrintString` (`KismetStringLibrary.Concat_StrStr` "Pokémon Asignado: " _pokemonname))
  (`SkeletalMeshComponent.SetSkeletalMeshAsset` (`self.Mesh`) _pokemonmesh)
  (`SkeletalMeshComponent.SetAnimInstanceClass` (`self.Mesh`) _animationblueprint))

(fn `UserConstructionScript`)