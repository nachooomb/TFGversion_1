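; Player controller for combat that locks look input, shows the mouse cursor and provides hold-to-skip for the intro cinematic.
; Pressing any key during a specific CombatManager state shows a skip prompt widget and starts a short timer, whose progress Tick feeds to the widget.
; Finishing the hold tells the manager to skip the cinematic, while releasing early cancels the timer; both remove the prompt.
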(event `self.ReceiveBeginPlay`
  (`self.SetIgnoreLookInput` true)
  (`self.SetIgnoreMoveInput` false)
  (set `self.bShowMouseCursor` true)
  (bind _returnvalue (`GameplayStatics.GetActorOfClass` "/Game/test001/Blueprints/Combat/BP_CombatManager.BP_CombatManager_C"))
  (`/Engine/EditorBlueprintResources/StandardMacros.IsValid` _returnvalue
    (:`Is Valid`
      (set `self.CombatManagerRef` _returnvalue))))

(event `Key|AnyKey`
  (params (Key :type "Key Structure"))
  (bind _combatmanagerref (`self.CombatManagerRef`))
  (:`Pressed`
    (set `self.bIsHoldingSkipKey` true)
    (`/Engine/EditorBlueprintResources/StandardMacros.IsValid` _combatmanagerref
      (:`Is Valid`
        (if (`|EnumEquality` (`/Game/test001/Blueprints/Combat/BP_CombatManager.CombatState` _combatmanagerref) "NewEnumerator8")
          (bind _returnvalue (`|CreateWidget` "/Game/test001/Blueprints/UI/Widgets/Skip/WB_SkipPrompt.WB_SkipPrompt_C" self))
          (bind _output_get (set `self.SkipPromptWidgetRef` _returnvalue))
          (`UserWidget.AddToViewport` _output_get 0)
          (bind _returnvalue_2 (`KismetSystemLibrary.K2_SetTimerDelegate` (`|CreateDelegate` :!event `OnHoldToSkipFinished`) 1.25))
          (set `self.SkipTimerHandle` _returnvalue_2)))))
  (:`Released`
    (set `self.bIsHoldingSkipKey` false)
    (`KismetSystemLibrary.K2_ClearAndInvalidateTimerHandle` (`self.SkipTimerHandle`))
    (`self.CleanUpSkipPrompt`)))

(event `OnHoldToSkipFinished`
  (bind _combatmanagerref (`self.CombatManagerRef`))
  (`/Engine/EditorBlueprintResources/StandardMacros.IsValid` _combatmanagerref
    (:`Is Valid`
      (`/Game/test001/Blueprints/Combat/BP_CombatManager.SkipIntroCinematic` _combatmanagerref)
      (`self.CleanUpSkipPrompt`))))

(event `self.ReceiveTick`
  (params (DeltaSeconds :type "Float (single-precision)"))
  (if (`self.bIsHoldingSkipKey`)
    (`/Engine/EditorBlueprintResources/StandardMacros.IsValid` (`self.SkipPromptWidgetRef`)
      (:`Is Valid`
        (`/Game/test001/Blueprints/UI/Widgets/Skip/WB_SkipPrompt.UpdateProgress` (`self.SkipPromptWidgetRef`) (/ (`KismetSystemLibrary.K2_GetTimerElapsedTimeHandle` (`self.SkipTimerHandle`)) 1.25))))))

(fn `CleanUpSkipPrompt`
  (bind _skippromptwidgetref (`self.SkipPromptWidgetRef`))
  (`/Engine/EditorBlueprintResources/StandardMacros.IsValid` _skippromptwidgetref
    (:`Is Valid`
      (`Widget.RemoveFromParent` _skippromptwidgetref)
      (set `self.SkipPromptWidgetRef` null))))

(fn `UserConstructionScript`)