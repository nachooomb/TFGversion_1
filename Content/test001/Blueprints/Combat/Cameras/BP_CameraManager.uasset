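; Combat camera manager that switches the player's view between default, player, enemy and dynamic cine cameras and controls their focus.
; SwitchToView blends the view target to the chosen camera and records it as the active one.
; FocusOnTarget snaps aperture and focus distance to a target on the current view camera.
; While focus tracking is on, Tick smoothly interpolates the active camera's manual focus distance toward the tracked actor.
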(event `self.ReceiveBeginPlay`
  (set `self.PlayerController` (`GameplayStatics.GetPlayerController` 0))
  (bind _ascine_camera_actor (cast `CineCameraActor` (`Controller.GetViewTarget` (`self.PlayerController`))))
  (set `self.ActiveCineCamera` _ascine_camera_actor))

(event `self.ReceiveTick`
  (params (DeltaSeconds :type "Float (single-precision)"))
  (bind _activecinecamera (`self.ActiveCineCamera`))
  (set `self.Delta Seconds` DeltaSeconds)
  (if (`self.bIsTrackingFocus`)
    (`/Engine/EditorBlueprintResources/StandardMacros.IsValid` _activecinecamera
      (:`Is Valid`
        (set `CineCameraComponent.FocusSettings` (make `CameraFocusSettings` "Manual" (`KismetMathLibrary.FInterpTo` (`.ManualFocusDistance` (break `CameraFocusSettings` (`CineCameraComponent.FocusSettings` (`CineCameraActor.GetCineCameraComponent` _activecinecamera)))) (`KismetMathLibrary.Vector_Distance` (`self.K2_GetActorLocation` (`self.TargetToFocus`)) (`SceneComponent.K2_GetComponentLocation` (`Actor.RootComponent` (`self.ActiveCineCamera`)))) (`self.Delta Seconds`) (`self.FocusInterpolationSpeed`))) (`CineCameraActor.GetCineCameraComponent` (`self.ActiveCineCamera`)))))))

(fn `FocusOnTarget`
  (params (TargetToFocus :type "Actor Object Reference") (`Current Aperture` :type "Float (single-precision)"))
  (locals (Local_ActiveCamera :type "CineCameraActor Object Reference"))
  (bind _ascine_camera_actor (cast `CineCameraActor` (`Controller.GetViewTarget` (`self.PlayerController`))))
  (set `local.Local_ActiveCamera` _ascine_camera_actor)
  (set `self.TargetToFocus` TargetToFocus)
  (set `CineCameraComponent.CurrentAperture` `Current Aperture` (`CineCameraActor.GetCineCameraComponent` (`local.Local_ActiveCamera`)))
  (set `CineCameraComponent.FocusSettings` (make `CameraFocusSettings` "Manual" (`KismetMathLibrary.Vector_Distance` (`self.K2_GetActorLocation` (`self.TargetToFocus`)) (`SceneComponent.K2_GetComponentLocation` (`Actor.RootComponent` (`local.Local_ActiveCamera`))))) (`CineCameraActor.GetCineCameraComponent` (`local.Local_ActiveCamera`))))

(fn `StartFocusTracking`
  (params (NewTarget :type "Actor Object Reference"))
  (set `self.TargetToFocus` NewTarget)
  (set `self.bIsTrackingFocus` true))

(fn `StopFocusTracking`
  (set `self.bIsTrackingFocus` false))

(fn `SwitchToView`
  (params (ViewToActivate :type "/Game/test001/Data/Enums/E_Cameras/E_CameraViews Enum" :default "NewEnumerator0"))
  (bind _defaultviewcamera (`self.DefaultViewCamera`))
  (bind _enemyviewcamera (`self.EnemyViewCamera`))
  (bind _playerviewcamera (`self.PlayerViewCamera`))
  (bind _dynamicviewcamera (`self.DynamicViewCamera`))
  (switch `/Game/test001/Data/Enums/E_Cameras/E_CameraViews` ViewToActivate
    (:`NewEnumerator0`
      (`PlayerController.SetViewTargetWithBlend` (`GameplayStatics.GetPlayerController` 0) _defaultviewcamera 1.0 "VTBlend_EaseIn" 0.0 false)
      (set `self.ActiveCineCamera` _defaultviewcamera))
    (:`NewEnumerator1`
      (`PlayerController.SetViewTargetWithBlend` (`self.PlayerController`) _playerviewcamera 1.0 "VTBlend_EaseIn" 0.0 false)
      (set `self.ActiveCineCamera` _playerviewcamera))
    (:`NewEnumerator2`
      (`PlayerController.SetViewTargetWithBlend` (`self.PlayerController`) _enemyviewcamera 1.0 "VTBlend_EaseIn" 0.0 true)
      (set `self.ActiveCineCamera` _enemyviewcamera))
    (:`NewEnumerator3`
      (`PlayerController.SetViewTargetWithBlend` (`self.PlayerController`) _dynamicviewcamera 1.0 "VTBlend_EaseInOut" 0.0 false)
      (set `self.ActiveCineCamera` _dynamicviewcamera))))

(fn `UserConstructionScript`)