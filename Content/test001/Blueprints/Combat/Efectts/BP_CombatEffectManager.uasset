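; Actor Blueprint that manages combat effects for a Pokémon-style battle, currently unfinished.
; ProcessAndApplyEffects filters effects by trigger but does not yet apply them or check their conditions.
; AreAllConditionsMet routes type, status and held-item conditions to subgraphs that test the user, selected target or last attacker, with optional negation.
; Failed checks print a red Spanish debug message, worded for type mismatch in all three.
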(fn `AreAllConditionsMet`
  (params (Conditions :type "Array of /Game/test001/Data/Structures/-111/BattleEffects/BattleEffectsStructures/S_EffectCondition Structure") (Context :type "/Game/test001/Data/Structures/-111/S_EffectExecutionContext Structure"))
  (returns (Result :type Boolean))
  (locals (Local_EffectSourcePokemon :type "/Game/test001/Blueprints/Pokemon/BP_Pokemon Object Reference") (Local_EffectSourceMoves :type "/Game/test001/Data/Structures/DataTables/RawDataStructs/S_PokemonMoves Structure") (Local_EffectSourceAbility :type "/Game/test001/Data/Structures/DataTables/RawDataStructs/S_PokemonAbilities Structure") (Local_EffectSourceItem :type "/Game/test001/Data/Structures/DataTables/RawDataStructs/S_Items Structure") (Local_PrimaryTarget :type "/Game/test001/Blueprints/Pokemon/BP_Pokemon Object Reference") (Local_LastAttacker :type "/Game/test001/Blueprints/Pokemon/BP_Pokemon Object Reference") (RequiredItem :type Name) (ConditionType :type "/Game/test001/Data/Structures/-111/BattleEffects/BattleEffectsEnums/Conditions/E_EffectConditionType Enum") (NegateCondition :type Boolean) (CheckTarget :type "/Game/test001/Data/Enums/E_Combat/E_EffectsTargets Enum") (ComparisonOperator :type "/Game/test001/Data/Structures/-111/BattleEffects/BattleEffectsEnums/Conditions/E_ComparisonOperator Enum") (RequiredType :type "/Game/test001/Data/Enums/E_Pokemon/E_PokemonTypes Enum") (RequiredMoveClasses :type "/Game/test001/Data/Enums/E_Moves/E_MoveDamageClasses Enum") (RequiredPersistantStatus :type "/Game/test001/Data/Enums/E_Pokemon/E_PersistantStatus Enum") (RequiredVolatileStatus :type "/Game/test001/Data/Enums/E_Combat/E_VolatileStatus Enum") (RequiredStat :type "/Game/test001/Data/Enums/E_Combat/E_CombatPokemonStats Enum") (ComparisonValue :type "Float (double-precision)") (bConditionCheckResult :type Boolean :default true) (PokemonToCheck :type "/Game/test001/Blueprints/Pokemon/BP_Pokemon Object Reference") (FoundVolatileStatus :type Boolean) (FoundPersistanStatus :type Boolean))
  (bind (_effectsource_pokemon _effectsource_moves _effectsource_ability _effectsource_item _primarytarget _lastattacker _requireditem) (break `/Game/test001/Data/Structures/-111/S_EffectExecutionContext` Context))
  (set `local.Local_EffectSourcePokemon` _effectsource_pokemon)
  (set `local.Local_EffectSourceMoves` _effectsource_moves)
  (set `local.Local_EffectSourceAbility` _effectsource_ability)
  (set `local.Local_EffectSourceItem` _effectsource_item)
  (set `local.Local_PrimaryTarget` _primarytarget)
  (set `local.Local_LastAttacker` _lastattacker)
  (set `local.RequiredItem` _requireditem)
  (for _array_element Conditions
    (bind (_conditiontype _negatecondition _checktarget _comparisonoperator _requiredtype _requiredmoveclases _requiredpersistantstatus _requiredvolatilestatus _requiredstat _comparisonvalue) (break `/Game/test001/Data/Structures/-111/BattleEffects/BattleEffectsStructures/S_EffectCondition` _array_element))
    (set `local.ConditionType` _conditiontype)
    (set `local.NegateCondition` _negatecondition)
    (set `local.CheckTarget` _checktarget)
    (set `local.ComparisonOperator` _comparisonoperator)
    (set `local.RequiredType` _requiredtype)
    (set `local.RequiredMoveClasses` _requiredmoveclases)
    (set `local.RequiredPersistantStatus` _requiredpersistantstatus)
    (set `local.RequiredVolatileStatus` _requiredvolatilestatus)
    (set `local.RequiredStat` _requiredstat)
    (set `local.ComparisonValue` _comparisonvalue)
    (switch `/Game/test001/Data/Structures/-111/BattleEffects/BattleEffectsEnums/Conditions/E_EffectConditionType` _conditiontype
      (:`NewEnumerator0`
        (`self.TargetIsOfType`)
        (return false))
      (:`NewEnumerator1`
        (`self.TargetHasStatus`)
        (return false))
      (:`NewEnumerator2`
        (`self.TargetHasItems`)
        (return false))))
  (return true))

(fn `ProcessAndApplyEffects`
  (params (EffectsToApply :type "Array of /Game/test001/Data/Structures/-111/BattleEffects/BattleEffectsStructures/S_BattleEffects Structure") (Context :type "/Game/test001/Data/Structures/-111/S_EffectExecutionContext Structure") (CurrentTrigger :type "/Game/test001/Data/Enums/E_Combat/E_BattleEventTrigger Enum" :default "NewEnumerator56"))
  (for _array_element EffectsToApply
    (bind (_affectedvariables _applicationconditions _health _ability _type _stats _status _movepp _currentmoveproperties _helditem _activepokemon _pokemonform _field _battlefields _terrain _weather _effecttarget _effecttrigger) (break `/Game/test001/Data/Structures/-111/BattleEffects/BattleEffectsStructures/S_BattleEffects` _array_element))
    (if (`|EnumEquality` _effecttrigger CurrentTrigger)
      (switch `/Game/test001/Data/Enums/E_Combat/E_BattleEventTrigger` _effecttrigger))))

(fn `UserConstructionScript`)