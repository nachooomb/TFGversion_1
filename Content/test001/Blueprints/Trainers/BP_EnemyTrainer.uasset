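; Enemy trainer character that performs a presentation walk to a given destination.
; BeginPlay prints the trainer's name and caches the ABP_Manny anim instance.
; ExecutePresentationWalk sets an animation flag and slows movement for an AIMoveTo, restoring both and signaling completion only on success.
; InitializeDissolveMaterials creates and stores dynamic Quinn torso and legs materials, but is not called within this Blueprint.
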(event `self.ReceiveBeginPlay`
  (`KismetSystemLibrary.PrintString` (`KismetStringLibrary.Concat_StrStr` "Entrenador " (`self.TrainerName`)) true true (struct :`G` 0.66 :`B` 1.0 :`A` 1.0) 4.0)
  (set `self.AnimationBlueprint` "/Game/Characters/Mannequins/Animations/ABP_Manny.ABP_Manny_C")
  (bind _asabp_manny (cast `/Game/Characters/Mannequins/Animations/ABP_Manny` (`SkeletalMeshComponent.GetAnimInstance` (`self.Mesh`))))
  (set `self.AnimBPRef` _asabp_manny))

(event `ExecutePresentationWalk`
  (params (Destinaiton :type "Vector Structure"))
  (set `/Game/Characters/Mannequins/Animations/ABP_Manny.bIsDoingPresentationWalk` true (`self.AnimBPRef`))
  (set `CharacterMovementComponent.MaxWalkSpeed` 175.0 (`self.CharacterMovement`))
  (`|AIMoveTo` self Destinaiton null
    (:`OnSuccess`
      (set `/Game/Characters/Mannequins/Animations/ABP_Manny.bIsDoingPresentationWalk` false (`self.AnimBPRef`))
      (set `CharacterMovementComponent.MaxWalkSpeed` 600.0 (`self.CharacterMovement`))
      (`self.OnPresentationFinished`))))

(fn `InitializeDissolveMaterials`
  (bind _returnvalue (`PrimitiveComponent.CreateDynamicMaterialInstance` (`self.Mesh`) 1 "/Game/test001/VFX/Materials/Quinn/MI_Quinn_Torso.MI_Quinn_Torso" "Quinn_02"))
  (set `self.DMI_Torso` _returnvalue)
  (bind _returnvalue_2 (`PrimitiveComponent.CreateDynamicMaterialInstance` (`self.Mesh`) 0 "/Game/test001/VFX/Materials/Quinn/MI_Quinn_Legs.MI_Quinn_Legs" "None"))
  (set `self.DMI_HeadLegs` _returnvalue_2))

(fn `UserConstructionScript`)