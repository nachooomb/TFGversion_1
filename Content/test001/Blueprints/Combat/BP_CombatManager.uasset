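; Combat manager that sets up a Pokémon battle and drives its states, camera and menus.
; BeginPlay spawns both trainers, initializes the GameInstance team and spawns both Pokémon, the enemy reusing the player's first team entry.
; SetCombatState switches BP_CombatCamera views and fills move names on move selection.
; After a start delay it creates five menu widgets, shown singly via ShowMenu; selecting a move only prints its index.
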(event `self.ReceiveBeginPlay`
  (`self.SpawnTrainers`)
  (bind _asbp_game_instance (cast `/Game/test001/Blueprints/Core/BP_GameInstance` (`GameplayStatics.GetGameInstance`)))
  (`/Game/test001/Blueprints/Core/BP_GameInstance.InitializeTeam` _asbp_game_instance)
  (`self.SpawnPokemon`)
  (`self.SetCombatCamera`)
  (`self.SetCombatState` "NewEnumerator0")
  (`self.OnCombatStart`))

(event `OnCombatStart`
  (`KismetSystemLibrary.PrintString` "Inicio de combate completado" true true (struct :`R` 1.0 :`G` 1.0 :`A` 1.0))
  (`KismetSystemLibrary.Delay` 1.0)
  (`self.InstanciateMenus`)
  (`self.SetCombatState` "NewEnumerator1"))

(event `OnMoveSelected`
  (params (MoveIndex :type Integer))
  (`KismetSystemLibrary.PrintString` (`KismetStringLibrary.Concat_StrStr` "Movimiento Selecionado:" (`KismetStringLibrary.Conv_IntToString` MoveIndex)) true true (struct :`R` 1.0 :`B` 0.070268 :`A` 1.0)))

(fn `ChangeCameraPosition`
  (params (ViewName :type Name))
  (bind _combatcamera (`self.CombatCamera`))
  (bind _combatcamera_2 (`self.CombatCamera`))
  (bind _combatcamera_3 (`self.CombatCamera`))
  (bind _combatcamera_4 (`self.CombatCamera`))
  (`/Engine/EditorBlueprintResources/StandardMacros.IsValid` (`self.CombatCamera`)
    (:`Is Valid`
      (switch `name` ViewName
        (:`DefaultView`
          (`/Game/test001/Blueprints/Cameras/BP_CombatCamera.ChangeCameraView` _combatcamera_2 (`/Game/test001/Blueprints/Cameras/BP_CombatCamera.DefaultView` _combatcamera_2)))
        (:`PlayerView`
          (`/Game/test001/Blueprints/Cameras/BP_CombatCamera.ChangeCameraView` _combatcamera_3 (`/Game/test001/Blueprints/Cameras/BP_CombatCamera.PlayerView` _combatcamera_3)))
        (:`EnemyView`
          (`/Game/test001/Blueprints/Cameras/BP_CombatCamera.ChangeCameraView` _combatcamera_4 (`/Game/test001/Blueprints/Cameras/BP_CombatCamera.EnemyView` _combatcamera_4)))
        (:`DynamicView`
          (`/Game/test001/Blueprints/Cameras/BP_CombatCamera.ChangeCameraView` _combatcamera (`/Game/test001/Blueprints/Cameras/BP_CombatCamera.DynamicView` _combatcamera)))))
    (:`Is Not Valid`
      (`KismetSystemLibrary.PrintString` "Hello"))))

(fn `InstanciateMenus`
  (bind _returnvalue (`|CreateWidget` "/Game/test001/Blueprints/UI/Widgets/CombatMenus/WB_CombatMainMenu.WB_CombatMainMenu_C"))
  (bind _output_get (set `self.CombatMainMenu` _returnvalue))
  (`UserWidget.AddToViewport` _output_get 0)
  (`Widget.SetVisibility` _output_get "Collapsed")
  (bind _returnvalue_2 (`|CreateWidget` "/Game/test001/Blueprints/UI/Widgets/CombatMenus/WB_MoveMenu.WB_MoveMenu_C"))
  (bind _output_get_2 (set `self.MoveSelectionMenu` _returnvalue_2))
  (`UserWidget.AddToViewport` _output_get_2 0)
  (`Widget.SetVisibility` _output_get_2 "Collapsed")
  (bind _returnvalue_3 (`|CreateWidget` "/Game/test001/Blueprints/UI/Widgets/CombatMenus/WB_PkmnTeamMenu.WB_PkmnTeamMenu_C"))
  (bind _output_get_3 (set `self.PkmnTeamMenu` _returnvalue_3))
  (`UserWidget.AddToViewport` _output_get_3 0)
  (`Widget.SetVisibility` _output_get_3 "Collapsed")
  (bind _returnvalue_4 (`|CreateWidget` "/Game/test001/Blueprints/UI/Widgets/CombatMenus/WB_CombatStatusMenu.WB_CombatStatusMenu_C"))
  (bind _output_get_4 (set `self.CombatStatusMenu` _returnvalue_4))
  (`UserWidget.AddToViewport` _output_get_4 0)
  (`Widget.SetVisibility` _output_get_4 "Collapsed")
  (bind _returnvalue_5 (`|CreateWidget` "/Game/test001/Blueprints/UI/Widgets/CombatMenus/WB_ExitMenu.WB_ExitMenu_C"))
  (bind _output_get_5 (set `self.ExitMenu` _returnvalue_5))
  (`UserWidget.AddToViewport` _output_get_5 0)
  (`Widget.SetVisibility` _output_get_5 "Collapsed")
  (set `self.CurrentMenu` (`self.CombatMainMenu`))
  (`self.ShowMenu` "NewEnumerator0"))

(fn `SetCombatCamera`
  (bind _outactors (`GameplayStatics.GetAllActorsOfClass` "/Game/test001/Blueprints/Cameras/BP_CombatCamera.BP_CombatCamera_C"))
  (set `self.CombatCamera` (`|GetArrayItem` _outactors))
  (bind _asbp_combat_player_controller (cast `/Game/test001/Blueprints/Controllers/BP_CombatPlayerController` (`GameplayStatics.GetPlayerController` 0)))
  (`PlayerController.SetViewTargetWithBlend` _asbp_combat_player_controller (`self.CombatCamera`) 0.0 "VTBlend_Linear" 0.0 false))

(fn `SetCombatState`
  (params (NewState :type "/Game/test001/PKMN_Data/Enums/E_CombatState Enum" :default "NewEnumerator0"))
  (bind _playerpokemon (`self.PlayerPokemon`))
  (bind _output_get (set `self.CombatState` NewState))
  (switch `/Game/test001/PKMN_Data/Enums/E_CombatState` _output_get
    (:`NewEnumerator0`
      (`KismetSystemLibrary.PrintString` "Estado: Inicio Combate" true true (struct :`R` 0.999977 :`G` 1.0 :`A` 1.0))
      (`self.ChangeCameraPosition` "DefaultView"))
    (:`NewEnumerator1`
      (`KismetSystemLibrary.PrintString` "Estado: Selección de Movimiento" true true (struct :`R` 0.999977 :`G` 1.0 :`A` 1.0))
      (`self.ChangeCameraPosition` "DynamicView")
      ;[1 1 1] update move data
      (if (`KismetSystemLibrary.IsValid` _playerpokemon)
        (bind _returnvalue (message `/Game/test001/Blueprints/Interfaces/BPI_PokemonData.GetPokemonData` _playerpokemon))
        (`/Game/test001/Blueprints/UI/Widgets/CombatMenus/WB_MoveMenu.UpdateMoveNames` (`self.MoveSelectionMenu`) (`.Moves_18_7A1C3B0D4074C361EE3BA1A825A3F1BE` (break `/Game/test001/PKMN_Data/Structures/S_combatPKMN` _returnvalue)))
        (else
          (`KismetSystemLibrary.PrintString` "Error al acceder al Pokémon"))))
    (:`NewEnumerator2`
      (`KismetSystemLibrary.PrintString` "Estado: Movimiento del Jugador" true true (struct :`R` 0.999977 :`G` 1.0 :`A` 1.0))
      (`self.ChangeCameraPosition` "PlayerView"))
    (:`NewEnumerator3`
      (`KismetSystemLibrary.PrintString` "Estado: Movimiento Enemigo" true true (struct :`R` 0.999977 :`G` 1.0 :`A` 1.0))
      (`self.ChangeCameraPosition` "EnemyView"))
    (:`NewEnumerator4`
      (`KismetSystemLibrary.PrintString` "Estado: Cambio de Pokémon" true true (struct :`R` 0.999977 :`G` 1.0 :`A` 1.0)))
    (:`NewEnumerator5`
      (`KismetSystemLibrary.PrintString` "Estado: Fin del Combate" true true (struct :`R` 1.0 :`G` 1.0 :`A` 1.0)))))

(fn `ShowMenu`
  (params (MenuName :type "/Game/test001/PKMN_Data/Enums/E_CombatMenus Enum" :default "NewEnumerator0"))
  (`/Engine/EditorBlueprintResources/StandardMacros.IsValid` (`self.CurrentMenu`)
    (:`Is Valid`
      (`Widget.SetVisibility` (`self.CurrentMenu`) "Collapsed")
      (switch `/Game/test001/PKMN_Data/Enums/E_CombatMenus` MenuName
        (:`NewEnumerator0`
          (bind _output_get (set `self.CurrentMenu` (`self.CombatMainMenu`)))
          (`Widget.SetVisibility` _output_get "Visible"))
        (:`NewEnumerator1`
          (bind _output_get_2 (set `self.CurrentMenu` (`self.MoveSelectionMenu`)))
          (`Widget.SetVisibility` _output_get_2 "Visible"))
        (:`NewEnumerator2`
          (bind _output_get_3 (set `self.CurrentMenu` (`self.PkmnTeamMenu`)))
          (`Widget.SetVisibility` _output_get_3 "Visible"))
        (:`NewEnumerator3`
          (bind _output_get_4 (set `self.CurrentMenu` (`self.CombatStatusMenu`)))
          (`Widget.SetVisibility` _output_get_4 "Visible"))
        (:`NewEnumerator4`
          (bind _output_get_5 (set `self.CurrentMenu` (`self.ExitMenu`)))
          (`Widget.SetVisibility` _output_get_5 "Visible"))))
    (:`Is Not Valid`
      (`KismetSystemLibrary.PrintString` "Hello"))))

(fn `SpawnPokemon`
  (locals (Local_PlayerTeam :type "Array of /Game/test001/PKMN_Data/Structures/S_combatPKMN Structure") (Local_PokemonData :type "/Game/test001/PKMN_Data/Structures/S_combatPKMN Structure"))
  (bind _asbp_game_instance (cast `/Game/test001/Blueprints/Core/BP_GameInstance` (`GameplayStatics.GetGameInstance`)))
  (bind _output_get (set `local.Local_PlayerTeam` (`/Game/test001/Blueprints/Core/BP_GameInstance.PlayerTeam` _asbp_game_instance)))
  (if (`KismetArrayLibrary.Array_IsEmpty` _output_get)
    (`KismetSystemLibrary.PrintString` "El equipo está vacío o no encontrado" true true (struct :`R` 1.0 :`G` 0.007329 :`A` 1.0))
    (else
      (bind _output_get_2 (set `local.Local_PokemonData` (`|GetArrayItem` (`local.Local_PlayerTeam`))))
      (bind _returnvalue (`|SpawnActorFromClass` (`.PokemonClass_29_57384862445C48144B09F69DB333C9AC` (break `/Game/test001/PKMN_Data/Structures/S_combatPKMN` _output_get_2)) (`SceneComponent.K2_GetComponentToWorld` (`self.PlayerSpawnPoint`)) "Undefined" "MultiplyWithRoot" null null))
      (bind _output_get_3 (set `self.PlayerPokemon` _returnvalue))
      (if (`KismetSystemLibrary.IsValid` _output_get_3)
        (message `/Game/test001/Blueprints/Interfaces/BPI_PokemonData.SetPokemonData` _output_get_3 (`local.Local_PokemonData`))
        (bind _returnvalue_2 (message `/Game/test001/Blueprints/Interfaces/BPI_PokemonData.GetPokemonData` _output_get_3))
        (`KismetSystemLibrary.PrintString` (`KismetStringLibrary.Concat_StrStr` "Pokemon del jugador generado en BP_CombatManager: " (`.PokemonName_2_D07B2A324EF6628628040A863E139A85` (break `/Game/test001/PKMN_Data/Structures/S_combatPKMN` _returnvalue_2))))
        (bind _returnvalue_3 (`|SpawnActorFromClass` "/Game/test001/Blueprints/Pokemon/BP_Pokemon.BP_Pokemon_C" (`SceneComponent.K2_GetComponentToWorld` (`self.EnemySpawnPoint`)) "Undefined" "MultiplyWithRoot" null null))
        (bind _output_get_4 (set `self.EnemyPokemon` _returnvalue_3))
        (if (`KismetSystemLibrary.IsValid` _output_get_4)
          (message `/Game/test001/Blueprints/Interfaces/BPI_PokemonData.SetPokemonData` _output_get_4 (`local.Local_PokemonData`))
          (bind _returnvalue_4 (message `/Game/test001/Blueprints/Interfaces/BPI_PokemonData.GetPokemonData` _output_get_4))
          (`KismetSystemLibrary.PrintString` (`KismetStringLibrary.Concat_StrStr` "Pokemon del Enemigo generado en BP_CombatManager: " (`.PokemonName_2_D07B2A324EF6628628040A863E139A85` (break `/Game/test001/PKMN_Data/Structures/S_combatPKMN` _returnvalue_4))))
          (else
            (`KismetSystemLibrary.PrintString` "Error al generar Pokémon")))
        (else
          (`KismetSystemLibrary.PrintString` "Error al generar Pokémon"))))))

(fn `SpawnTrainers`
  (bind _returnvalue (`|SpawnActorFromClass` "/Game/test001/Blueprints/Trainers/BP_Trainer.BP_Trainer_C" (`SceneComponent.K2_GetComponentToWorld` (`self.PlayerTrainerPoint`)) "Undefined" "MultiplyWithRoot" null null))
  (set `self.PlayerTrainer` _returnvalue)
  (`KismetSystemLibrary.PrintString` "Entrenador del jugador generado" true true (struct :`R` 0.062745 :`G` 1.0 :`A` 1.0))
  (bind _returnvalue_2 (`|SpawnActorFromClass` "/Game/test001/Blueprints/Trainers/BP_Trainer.BP_Trainer_C" (`SceneComponent.K2_GetComponentToWorld` (`self.EnemyTrainerPoint`)) "Undefined" "MultiplyWithRoot" null null))
  (set `self.EnemyTrainer` _returnvalue_2)
  (`KismetSystemLibrary.PrintString` "Entrenador enemigo generado" true true (struct :`R` 1.0 :`B` 0.021888 :`A` 1.0)))

(fn `UserConstructionScript`)