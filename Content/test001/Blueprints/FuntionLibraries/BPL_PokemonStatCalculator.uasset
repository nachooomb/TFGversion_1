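; Blueprint function library that builds a Pokémon's final six-stat block from form base stats, level, IVs and EVs.
; CalculateFinalStats looks up the nature row in DT_Natures and feeds it to every per-stat helper except HP.
; Helpers hold floored stat formulas with 1.1/0.9 nature multipliers, though these expressions appear unconnected to any output.
; A missing nature row is unhandled, and the debug print is disconnected.
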(fn `CalculateFinalStats`
  (params (PokemonFormData :type "/Game/test001/Data/Structures/DataTables/RawDataStructs/S_PokemonForm Structure") (PokemonData :type "/Game/test001/Data/Structures/S_Pokemon Structure"))
  (returns (FinalStats :type "/Game/test001/Data/Structures/Sub_Structures/SS_StatBlock Structure"))
  (bind (_instanceid _nickname _formname _currentxp _level _ivs _evs _nature) (break `/Game/test001/Data/Structures/S_Pokemon` PokemonData))
  (bind (_hp _attack _defense _specialattack _specialdefense _speed) (break `/Game/test001/Data/Structures/Sub_Structures/SS_StatBlock` _ivs))
  (bind (_hp_2 _attack_2 _defense_2 _specialattack_2 _specialdefense_2 _speed_2) (break `/Game/test001/Data/Structures/Sub_Structures/SS_StatBlock` _evs))
  (bind (_hp_3 _attack_3 _defense_3 _specialattack_3 _specialdefense_3 _speed_3) (break `/Game/test001/Data/Structures/Sub_Structures/SS_StatBlock` (`.BaseStats_77_CF7BE0CB47AE66DD3B7E6588ED111788` (break `/Game/test001/Data/Structures/DataTables/RawDataStructs/S_PokemonForm` PokemonFormData))))
  (bind _returnvalue (`KismetMathLibrary.Conv_IntToDouble` _level))
  (bind _returnvalue_2 (`|GetDataTableRow` "/Game/test001/Data/Structures/1-S_teamBuilder/nature/DT_Natures.DT_Natures" (`KismetStringLibrary.Conv_StringToName` (`|GetEnumeratorNameAsString` _nature)))
    (:`then`
      (bind (_increasedstat _decreasedstat) (break `/Game/test001/Data/Structures/1-S_teamBuilder/nature/S_natureData` _returnvalue_2))
      (bind (_increasedstat_2 _decreasedstat_2) (break `/Game/test001/Data/Structures/1-S_teamBuilder/nature/S_natureData` _returnvalue_2))
      (bind (_increasedstat_3 _decreasedstat_3) (break `/Game/test001/Data/Structures/1-S_teamBuilder/nature/S_natureData` _returnvalue_2))
      (bind (_increasedstat_4 _decreasedstat_4) (break `/Game/test001/Data/Structures/1-S_teamBuilder/nature/S_natureData` _returnvalue_2))
      (bind (_increasedstat_5 _decreasedstat_5) (break `/Game/test001/Data/Structures/1-S_teamBuilder/nature/S_natureData` _returnvalue_2))
      (return (make `/Game/test001/Data/Structures/Sub_Structures/SS_StatBlock` (`KismetMathLibrary.FFloor` (+ (+ _returnvalue (`KismetMathLibrary.FFloor` (/ (* _returnvalue (+ (+ (* (`KismetMathLibrary.Conv_IntToDouble` _hp_3) 2.0) (`KismetMathLibrary.Conv_IntToDouble` _hp)) (`KismetMathLibrary.FFloor` (/ (`KismetMathLibrary.Conv_IntToDouble` _hp_2) 4.0)))) 100.0))) 10.0)) (`KismetMathLibrary.FFloor` (* (+ (/ (* (`KismetMathLibrary.Conv_IntToDouble` _level) (+ (* (`KismetMathLibrary.Conv_IntToDouble` _attack_3) 2.0) (`KismetMathLibrary.Conv_IntToDouble` _attack) (`KismetMathLibrary.FFloor` (/ (`KismetMathLibrary.Conv_IntToDouble` _attack_2) 4.0)))) 100.0) 5.0) (`KismetMathLibrary.SelectFloat` 1.1 (`KismetMathLibrary.SelectFloat` 0.9 1.0 (`|EnumEquality` _decreasedstat "NewEnumerator1")) (`|EnumEquality` _increasedstat "NewEnumerator1")))) (`KismetMathLibrary.FFloor` (* (+ (/ (* (`KismetMathLibrary.Conv_IntToDouble` _level) (+ (* (`KismetMathLibrary.Conv_IntToDouble` _defense_3) 2.0) (`KismetMathLibrary.Conv_IntToDouble` _defense) (`KismetMathLibrary.FFloor` (/ (`KismetMathLibrary.Conv_IntToDouble` _defense_2) 4.0)))) 100.0) 5.0) (`KismetMathLibrary.SelectFloat` 1.1 (`KismetMathLibrary.SelectFloat` 0.9 1.0 (`|EnumEquality` _decreasedstat_2 "NewEnumerator2")) (`|EnumEquality` _increasedstat_2 "NewEnumerator2")))) (`KismetMathLibrary.FFloor` (* (+ (/ (* (`KismetMathLibrary.Conv_IntToDouble` _level) (+ (* (`KismetMathLibrary.Conv_IntToDouble` _specialattack_3) 2.0) (`KismetMathLibrary.Conv_IntToDouble` _specialattack) (`KismetMathLibrary.FFloor` (/ (`KismetMathLibrary.Conv_IntToDouble` _specialattack_2) 4.0)))) 100.0) 5.0) (`KismetMathLibrary.SelectFloat` 1.1 (`KismetMathLibrary.SelectFloat` 0.9 1.0 (`|EnumEquality` _decreasedstat_3 "NewEnumerator3")) (`|EnumEquality` _increasedstat_3 "NewEnumerator3")))) (`KismetMathLibrary.FFloor` (* (+ (/ (* (`KismetMathLibrary.Conv_IntToDouble` _level) (+ (* (`KismetMathLibrary.Conv_IntToDouble` _specialdefense_3) 2.0) (`KismetMathLibrary.Conv_IntToDouble` _specialdefense) (`KismetMathLibrary.FFloor` (/ (`KismetMathLibrary.Conv_IntToDouble` _specialdefense_2) 4.0)))) 100.0) 5.0) (`KismetMathLibrary.SelectFloat` 1.1 (`KismetMathLibrary.SelectFloat` 0.9 1.0 (`|EnumEquality` _decreasedstat_4 "NewEnumerator4")) (`|EnumEquality` _increasedstat_4 "NewEnumerator4")))) (`KismetMathLibrary.FFloor` (* (+ (/ (* (`KismetMathLibrary.Conv_IntToDouble` _level) (+ (* (`KismetMathLibrary.Conv_IntToDouble` _speed_3) 2.0) (`KismetMathLibrary.Conv_IntToDouble` _speed) (`KismetMathLibrary.FFloor` (/ (`KismetMathLibrary.Conv_IntToDouble` _speed_2) 4.0)))) 100.0) 5.0) (`KismetMathLibrary.SelectFloat` 1.1 (`KismetMathLibrary.SelectFloat` 0.9 1.0 (`|EnumEquality` _decreasedstat_5 "NewEnumerator5")) (`|EnumEquality` _increasedstat_5 "NewEnumerator5")))))))))